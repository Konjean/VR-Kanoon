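; Cannon actor that animates itself on BeginPlay and then fires projectiles continuously.
; A timeline lerps the lever from its starting rotation to an end rotation, then a second timeline swings the cannon pivot to its end rotation.
; Once aimed, it loops forever, spawning two scaled-up projectiles at the shooting point's location and rotation, then waiting on a short delay.
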(event EventBeginPlay
  (bind _shooting_point (Variables|Default|GetShooting%20Point))
  (bind _returnvalue (Transformation|GetWorldTransform _shooting_point))
  (Variables|Default|SetLever%20First%20Rotation (Variables|/Script/Engine.SceneComponent|GetRelativeRotation (Variables|Default|GetLever%20Rotation)))
  (Variables|Default|SetCannonFirstRotation (Variables|/Script/Engine.SceneComponent|GetRelativeRotation (Variables|Default|GetCannon%20Rotation%20Point)))
  (bind _newtrack_0 (Timeline|Timeline Play)
    (:Update
      (Transformation|SetRelativeRotation (Variables|Default|GetLever%20Rotation) (Math|Rotator|Lerp(Rotator) (Variables|Default|GetLever%20First%20Rotation) (Variables|Default|GetLever%20End%20Rotation) _newtrack_0) false false))
    (:Finished
      (bind _newtrack_0_2 (Timeline|Timeline_0 Play)
        (:Update
          (Transformation|SetRelativeRotation (Variables|Default|GetCannon%20Rotation%20Point) (Math|Rotator|Lerp(Rotator) (Variables|Default|GetCannonFirstRotation) (Variables|Default|GetCannonEndRotation) _newtrack_0_2) false false))
        (:Finished
          (Game|SpawnActorfromClass "/Game/VRTemplate/Blueprints/Projectile.Projectile_C" (Math|Transform|MakeTransform (.location _returnvalue) (.rotation _returnvalue) "5.000000,5.000000,5.000000") "Undefined" "MultiplyWithRoot" 0 0 :!label _label)
          (Game|SpawnActorfromClass "/Game/VRTemplate/Blueprints/Projectile.Projectile_C" (Math|Transform|MakeTransform (.location _returnvalue) (.rotation _returnvalue) "5.000000,5.000000,5.000000") "Undefined" "MultiplyWithRoot" 0 0)
          (Utilities|FlowControl|Delay 2.0)
          (goto _label))))))

(event Collision|EventActorBeginOverlap
  (params (OtherActor :type Actor%20Object%20Reference)))

(event EventTick
  (params (DeltaSeconds :type Float%20%28single-precision%29)))

(fn ConstructionScript)